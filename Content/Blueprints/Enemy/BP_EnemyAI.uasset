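; Enemy character Blueprint that detects the player, fires a rifle and ragdolls on death.
; AI perception feeds target and line-of-sight updates to the AI controller, clearing the target after a short timer when sight is lost.
; A data table row drives weapon attachment, fire effects and projectile spawning; the debug line trace's result is unused.
; Damage plays random hit montages until health runs out, and a timeline eases walk speed changes.
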(event OnTargetPerceptionUpdated(AIPerception)
  (params (Actor :type Actor%20Object%20Reference) (Stimulus :type AI%20Stimulus%20Structure))
  (bind _output_get (Variables|Default|SetPerceivedActor Actor))
  (if (Math|Boolean|ANDBoolean (== _output_get (Variables|Default|GetPlayerCharacter)) (Utilities|Struct|BreakAIStimulus Stimulus) (Variables|Default|GetIsAlive?))
    (Variables|Default|SetPerceivedActor (Variables|Default|GetPlayerCharacter))
    (Utilities|Time|ClearandInvalidateTimerbyHandle (Variables|Default|GetTargetLostTime))
    (Class|BPEnemyAIConInterface|UpdateTargetActorKey(Message) (Variables|Default|GetAIController) (Variables|Default|GetPerceivedActor))
    (Class|BPEnemyAIConInterface|UpdateHasLineOfSightKey(Message) (Variables|Default|GetAIController) true)
    (elif (== (Variables|Default|GetPlayerCharacter) (Variables|Default|GetPerceivedActor))
      (bind _returnvalue (Utilities|Time|SetTimerbyEvent (delegate Custom|TargetLost) 5.0))
      (Variables|Default|SetTargetLostTime _returnvalue)
      (Class|BPEnemyAIConInterface|UpdateHasLineOfSightKey(Message) (Variables|Default|GetAIController) false))))

(event Custom|TargetLost
  (Class|BPEnemyAIConInterface|UpdateTargetActorKey(Message) (Variables|Default|GetAIController)))

(event EventBeginPlay
  (bind _returnvalue (Utilities|GetDataTableRow "/Game/Blueprints/Weapons/WeaponDataTable.WeaponDataTable" "Rifle")
    (:then
      (Transformation|AttachComponentToComponent (Variables|Default|GetWeaponMesh) (Variables|Character|GetMesh) (Utilities|Struct|BreakWeaponsStructure _returnvalue) "KeepRelative" "KeepRelative" "KeepRelative" true)
      (Variables|Default|SetPlayerCharacter (Game|GetPlayerCharacter 0))
      (Variables|Default|SetAIController (Pawn|GetController))
      (bind _returnvalue_2 (UserInterface|CreateWidget "/Game/UMG/UI_ExClamationMark.UI_ExClamationMark_C" (Game|GetPlayerController 0)))
      (Variables|Default|SetExclamationMark _returnvalue_2))))

(event EventAttack
  (bind _weaponmesh (Variables|Default|GetWeaponMesh))
  (if (Variables|Default|GetIsAlive?)
    (bind _returnvalue (Utilities|GetDataTableRow "/Game/Blueprints/Weapons/WeaponDataTable.WeaponDataTable" "Rifle")
      (:then
        (Utilities|FlowControl|Sequence
          (:then_0
            (Audio|PlaySound2D (.FireSound (Utilities|Struct|BreakWeaponsStructure _returnvalue)) 1.0 1.0 0.0 0 0))
          (:then_1
            (Animation|PlayAnimMontage (.FireMOntage (Utilities|Struct|BreakWeaponsStructure _returnvalue)) 0.1 "None"))
          (:then_2
            (Effects|SpawnEmitterAttached (.MuzzleFlash (Utilities|Struct|BreakWeaponsStructure _returnvalue)) (Variables|Default|GetWeaponMesh) (.MuzzleFlashSocketName (Utilities|Struct|BreakWeaponsStructure _returnvalue))))
          (:then_3
            (Game|SpawnActorfromClass (.AmmoClass (Utilities|Struct|BreakWeaponsStructure _returnvalue)) (Transformation|GetSocketTransform _weaponmesh (.AmmoSocketName (Utilities|Struct|BreakWeaponsStructure _returnvalue)) "RTS_World") "AlwaysSpawn" 0 0)
            (Collision|LineTraceByChannel (Transformation|GetSocketLocation _weaponmesh (.MuzzleFlashSocketName (Utilities|Struct|BreakWeaponsStructure _returnvalue))) (+ (Transformation|GetSocketLocation _weaponmesh (.MuzzleFlashSocketName (Utilities|Struct|BreakWeaponsStructure _returnvalue))) (* (Math|Vector|GetForwardVector (Transformation|GetSocketRotation _weaponmesh (.MuzzleFlashSocketName (Utilities|Struct|BreakWeaponsStructure _returnvalue)))) 1e+04)) "TraceTypeQuery1" false 0 "ForDuration")))))))

(event EventChangeWalkSpeed
  (params (Speed :type Float%20%28single-precision%29))
  (Timeline|UpdateTimeline PlayFromStart
    (:Update
      (Variables|/Script/Engine.CharacterMovementComponent|SetMaxWalkSpeed (Variables|Character|GetCharacterMovement) (Math|Interpolation|FInterpTo (Variables|/Script/Engine.CharacterMovementComponent|GetMaxWalkSpeed (Variables|Character|GetCharacterMovement)) Speed (Utilities|Time|GetWorldDeltaSeconds) 5.0)))))

(event Game|Damage|EventAnyDamage
  (params (Damage :type Float%20%28single-precision%29) (DamageType :type Damage%20Type%20Object%20Reference) (InstigatedBy :type Controller%20Object%20Reference) (DamageCauser :type Actor%20Object%20Reference))
  (bind _output_get (Variables|Default|SetHealth (- (Variables|Default|GetHealth) Damage)))
  (if (<= _output_get 0.0)
    (Pawn|Components|CharacterMovement|DisableMovement (Variables|Character|GetCharacterMovement))
    (Physics|SetSimulatePhysics (Variables|Character|GetMesh) true)
    (Collision|SetCollisionEnabled (Variables|Collision|GetCapsuleComponent) "NoCollision")
    (Variables|Default|SetIsAlive? false)
    (else
      (Animation|PlayAnimMontage (Utilities|Array|Get(acopy) (Variables|Default|GetHitMontages) (Math|Random|RandomIntegerinRange 0 3)) 2.0 "None"))))

(fn ConstructionScript)